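; BP_ENV is an environment actor whose Opa component shows a tintable layer material, MAT_EnvCoucheOpa.
; The construction script creates a dynamic material instance on Opa and sets its Color parameter from the Color variable.
; At BeginPlay it moves itself to 1000 units below the world origin and stores a fresh dynamic instance.
; The ColorChange event pushes the current Color value to that stored instance.
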(event `self.ReceiveBeginPlay`
  (`self.K2_SetActorLocation` (0.0 0.0 -1000.0))
  (bind _returnvalue (`PrimitiveComponent.CreateDynamicMaterialInstance` (`self.Opa`) 0 "/Game/Materials/MAT_EnvCoucheOpa.MAT_EnvCoucheOpa"))
  (set `self.DynamicMatEnv` _returnvalue))

(event `ColorChange`
  (`MaterialInstanceDynamic.SetVectorParameterValue` (`self.DynamicMatEnv`) "Color" (`self.Color`)))

(fn `UserConstructionScript`
  (bind _returnvalue (`PrimitiveComponent.CreateDynamicMaterialInstance` (`self.Opa`) 0 "/Game/Materials/MAT_EnvCoucheOpa.MAT_EnvCoucheOpa"))
  (`MaterialInstanceDynamic.SetVectorParameterValue` _returnvalue "Color" (`self.Color`)))