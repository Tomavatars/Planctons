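; Game controller for a three-level plankton game that starts and stops game mode, shows the victory widget and drives enemy spawning.
; BeginPlay stores difficulty, caches the camera, Plancton_Manager and main plankton, then starts level 1.
; One-shot level events have the manager spawn difficulty-scaled Plasticos and one Robota at each level's height.
; Waves spawns more Plasticos, with count and speed set by wave and camera level; GameLoose is empty.
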(event `BeginPlay`
  (params (Difficulty :type Integer))
  ;[1 1 1] BeginPlay
  (set `self.Difficulty` Difficulty)
  (bind _outactors (`GameplayStatics.GetAllActorsOfClass` "/Game/Blueprints/Camera/BP_MainCamera.BP_MainCamera_C"))
  (set `self.RefCamera` (`KismetArrayLibrary.Array_Get` _outactors))
  (bind _outactors_2 (`GameplayStatics.GetAllActorsOfClass` "/Game/Blueprints/Actors/Plancton_Manager.Plancton_Manager_C"))
  (set `self.RefManager` (`KismetArrayLibrary.Array_Get` _outactors_2))
  (bind _outactors_3 (`GameplayStatics.GetAllActorsOfClass` "/Game/Blueprints/Actors/BP_MainPlancton.BP_MainPlancton_C"))
  (`|ExecutionSequence`
    (:`then_0`
      (set `self.RefMainPlancton` (`KismetArrayLibrary.Array_Get` _outactors_3))
      (`/Game/Blueprints/Camera/BP_MainCamera.RefGameMode` (`self.RefCamera`) true)
      (`self.MakeGameLv1`))
    (:`then_1`
      (for _array_element _outactors_3
        (`/Game/Blueprints/Actors/BP_MainPlancton.GameOn` _array_element)))))

(event `GameWon`
  (bind _returnvalue (`|CreateWidget` "/Game/Widgets/WID_Victoire.WID_Victoire_C"))
  (`UserWidget.AddToViewport` _returnvalue 0))

(event `UndoGameMode`
  (`/Game/Blueprints/Actors/BP_MainPlancton.GameOff` (`self.RefMainPlancton`))
  (`/Game/Blueprints/Camera/BP_MainCamera.RefGameMode` (`self.RefCamera`) false))

(event `GameLoose`)

(event `MakeGameLv1`
  (bind _refmanager (`self.RefManager`))
  (`/Engine/EditorBlueprintResources/StandardMacros.DoOnce` false :!label _label
    (:`Completed`
      (set `self.RobotaMinSpeed` 3.0)
      (set `self.RobotaMaxSpeed` 6.0)
      (set `self.PlasticoMinSpeed` 2.0)
      (set `self.PlasticoMaxSpeed` 4.0)
      (`/Game/Blueprints/Actors/BP_MainPlancton.GameOn` (`self.RefMainPlancton`))
      (bind _output_get (set `self.ZValue` 2000.0))
      (`/Game/Blueprints/Actors/Plancton_Manager.Spawn-Plastico` _refmanager "NewEnumerator0" _output_get "NewEnumerator0" (select `int` (`self.Difficulty`) :`0` 2 :`1` 2 :`2` 3 :`3` 3 :`4` 4 :`5` 4) (`self.PlasticoMinSpeed`) (`self.PlasticoMaxSpeed`))
      (`/Game/Blueprints/Actors/Plancton_Manager.Plastica-Robota-Spawn` _refmanager "NewEnumerator0" _output_get "NewEnumerator0" 1 (`self.RobotaMinSpeed`) (`self.RobotaMaxSpeed`) (`self.Difficulty`)))))

(event `ResetGame`
  (goto _label :!via `Reset`))

(event `MakeGameLv2`
  (bind _refmanager (`self.RefManager`))
  (`/Engine/EditorBlueprintResources/StandardMacros.DoOnce` false
    (:`Completed`
      (set `self.RobotaMinSpeed` 3.0)
      (set `self.RobotaMaxSpeed` 6.0)
      (set `self.PlasticoMinSpeed` 4.0)
      (set `self.PlasticoMaxSpeed` 6.0)
      (bind _output_get (set `self.ZValue` 1000.0))
      (`/Game/Blueprints/Actors/Plancton_Manager.Spawn-Plastico` _refmanager "NewEnumerator0" _output_get "NewEnumerator1" (select `int` (`self.Difficulty`) :`0` 3 :`1` 3 :`2` 4 :`3` 4 :`4` 5 :`5` 5) (`self.PlasticoMinSpeed`) (`self.PlasticoMaxSpeed`))
      (`/Game/Blueprints/Actors/Plancton_Manager.Plastica-Robota-Spawn` _refmanager "NewEnumerator0" _output_get "NewEnumerator1" 1 (`self.RobotaMinSpeed`) (`self.RobotaMaxSpeed`) (`self.Difficulty`)))))

(event `MakeGameLv3`
  (bind _refmanager (`self.RefManager`))
  (`/Engine/EditorBlueprintResources/StandardMacros.DoOnce` false
    (:`Completed`
      (set `self.RobotaMinSpeed` 4.0)
      (set `self.RobotaMaxSpeed` 8.0)
      (set `self.PlasticoMinSpeed` 6.0)
      (set `self.PlasticoMaxSpeed` 8.0)
      (bind _output_get (set `self.ZValue` 0.0))
      (`/Game/Blueprints/Actors/Plancton_Manager.Spawn-Plastico` _refmanager "NewEnumerator2" _output_get "NewEnumerator2" (select `int` (`self.Difficulty`) :`0` 4 :`1` 4 :`2` 5 :`3` 5 :`4` 6 :`5` 6) (`self.PlasticoMinSpeed`) (`self.PlasticoMaxSpeed`))
      (`/Game/Blueprints/Actors/Plancton_Manager.Plastica-Robota-Spawn` _refmanager "NewEnumerator0" _output_get "NewEnumerator2" 1 (`self.RobotaMinSpeed`) (`self.RobotaMaxSpeed`) (`self.Difficulty`)))))

(event `Waves`
  (bind _wavesref (`self.WavesRef`))
  ;[1 1 1] Waves
  (switch `/Game/Blueprints/Camera/EN_LevelCam` (`/Game/Blueprints/Camera/BP_MainCamera.Level` (`self.RefCamera`))
    (:`NewEnumerator0`
      (set `self.ToSpawn` (select `/Game/Blueprints/EN_Waves` _wavesref :`NewEnumerator0` 2 :`NewEnumerator1` 3 :`NewEnumerator2` 4 :`NewEnumerator3` 5 :`NewEnumerator4` 6))
      (set `self.PlasticoMinSpeed` (select `/Game/Blueprints/EN_Waves` _wavesref :`NewEnumerator0` 2.0 :`NewEnumerator1` 2.0 :`NewEnumerator2` 2.5 :`NewEnumerator3` 2.5 :`NewEnumerator4` 2.5 :!type "Float (single-precision)"))
      (set `self.PlasticoMaxSpeed` (select `/Game/Blueprints/EN_Waves` _wavesref :`NewEnumerator0` 3.0 :`NewEnumerator1` 4.0 :`NewEnumerator2` 5.0 :`NewEnumerator3` 5.0 :`NewEnumerator4` 5.0 :!type "Float (single-precision)"))
      (set `self.ZValue` 2000.0))
    (:`NewEnumerator1`
      (set `self.ToSpawn` (select `/Game/Blueprints/EN_Waves` _wavesref :`NewEnumerator0` 3 :`NewEnumerator1` 4 :`NewEnumerator2` 5 :`NewEnumerator3` 6 :`NewEnumerator4` 7))
      (set `self.PlasticoMinSpeed` (select `/Game/Blueprints/EN_Waves` _wavesref :`NewEnumerator0` 4.0 :`NewEnumerator1` 4.0 :`NewEnumerator2` 5.0 :`NewEnumerator3` 5.0 :`NewEnumerator4` 5.0 :!type "Float (single-precision)"))
      (set `self.PlasticoMaxSpeed` (select `/Game/Blueprints/EN_Waves` _wavesref :`NewEnumerator0` 6.0 :`NewEnumerator1` 6.0 :`NewEnumerator2` 7.0 :`NewEnumerator3` 7.0 :`NewEnumerator4` 7.0 :!type "Float (single-precision)"))
      (set `self.ZValue` 1000.0))
    (:`NewEnumerator2`
      (set `self.ToSpawn` (select `/Game/Blueprints/EN_Waves` _wavesref :`NewEnumerator0` 4 :`NewEnumerator1` 5 :`NewEnumerator2` 6 :`NewEnumerator3` 7 :`NewEnumerator4` 8))
      (set `self.PlasticoMinSpeed` (select `/Game/Blueprints/EN_Waves` _wavesref :`NewEnumerator0` 6.0 :`NewEnumerator1` 6.0 :`NewEnumerator2` 7.0 :`NewEnumerator3` 7.0 :`NewEnumerator4` 7.0 :!type "Float (single-precision)"))
      (set `self.PlasticoMaxSpeed` (select `/Game/Blueprints/EN_Waves` _wavesref :`NewEnumerator0` 8.0 :`NewEnumerator1` 8.0 :`NewEnumerator2` 9.0 :`NewEnumerator3` 10.0 :`NewEnumerator4` 11.0 :!type "Float (single-precision)"))
      (set `self.ZValue` 0.0)))
  (`/Game/Blueprints/Actors/Plancton_Manager.Spawn-Plastico` (`self.RefManager`) "NewEnumerator0" (`self.ZValue`) (select `/Game/Blueprints/Camera/EN_LevelCam` (`/Game/Blueprints/Camera/BP_MainCamera.Level` (`self.RefCamera`)) :`NewEnumerator0` "NewEnumerator0" :`NewEnumerator1` "NewEnumerator1" :`NewEnumerator2` "NewEnumerator2" :!type "/Game/Blueprints/Actors/EN_Level Enum") (`self.ToSpawn`) (`self.PlasticoMinSpeed`) (`self.PlasticoMaxSpeed`)))