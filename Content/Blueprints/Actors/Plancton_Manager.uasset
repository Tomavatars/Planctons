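; Manager actor that spawns BP_MainPlancton actors for a target level, using rows from the Plancton_CSV data table.
; Spawn and SpawnKilled shuffle the row names and skip rows until type and level match, creating an initial batch or one same-type replacement at side offsets.
; Separate events spawn Plasticoplanctons and the Plastica Robota from named rows, and Destroy notifies all planctons.
; Delay-based loop macros stagger the batch spawns.
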(event `UpdateLoopKill`
  (bind _typerespwan (`self.TypeRespwan`))
  ;[1 1 1] Spawn Killed
  (if (< (`self.KilledIndex`) (`KismetArrayLibrary.Array_LastIndex` (stale `SpawnKilled` _outrownames))) :!label _label
    (bind _returnvalue (`|GetDataTableRow` "/Game/Blueprints/Actors/Plancton_CSV.Plancton_CSV" (`KismetArrayLibrary.Array_Get` (stale `SpawnKilled` _outrownames) (`self.KilledIndex`)))
      (:`then`
        (bind (_texture _normal _nom _famille _description _speed _type _level _nlevel _eleve) (break `/Game/Blueprints/Actors/STR_Plantons` _returnvalue))
        (if (== _type _typerespwan)
          (bind _output_get (set `self.ActorLevel` _nlevel))
          (if (== _output_get (`self.TargetedLevel`))
            (`self.UpdateIndexKill`)
            (`/Engine/EditorBlueprintResources/StandardMacros.FlipFlop`
              (:`A`
                (set `self.SpawnY` (`KismetMathLibrary.RandomFloatInRange` 0.0 900.0))
                (set `self.SpawnX` (`KismetMathLibrary.RandomFloatInRange` 500.0 600.0)))
              (:`B`
                (set `self.SpawnY` (`KismetMathLibrary.RandomFloatInRange` 0.0 -900.0))
                (set `self.SpawnX` (`KismetMathLibrary.RandomFloatInRange` -500.0 -600.0))))
            (`|SpawnActorFromClass` "/Game/Blueprints/Actors/BP_MainPlancton.BP_MainPlancton_C" (`KismetMathLibrary.MakeTransform` (`KismetMathLibrary.MakeVector` (`self.SpawnX`) (`self.SpawnY`) _level) (struct) (5.0 5.0 1.0)) "Undefined" "OverrideRootScale" null _level (/ _speed 4.0) _texture _type _normal (`KismetTextLibrary.Conv_StringToText` _nom) (`KismetTextLibrary.Conv_StringToText` _famille) (`KismetTextLibrary.Conv_StringToText` _description) _nlevel null (`KismetTextLibrary.Conv_StringToText` _eleve) false _typerespwan (`self.PlasticGameMode`) 4.0 6.0 false 3.0 6.0 5)
            (else
              (`self.UpdateIndexKill` :!label _label_2)
              (`self.UpdateLoopKill`)))
          (else
            (goto _label_2)))))))

(event `SpawnKilled`
  (params (TargetedLevel :type "/Game/Blueprints/Actors/EN_Level Enum") (TypeRespawn :type "/Game/Blueprints/Actors/EN_TypePlancton Enum"))
  (bind _forloopindexkilled (`self.ForLoopIndexKilled`))
  ;[1 1 1] Spawn Killed
  (set `self.TargetedLevel` TargetedLevel)
  (set `self.TypeRespwan` TypeRespawn)
  (set `self.KilledIndex` 0)
  (bind _outrownames (`DataTableFunctionLibrary.GetDataTableRowNames` "/Game/Blueprints/Actors/Plancton_CSV.Plancton_CSV"))
  (`KismetArrayLibrary.Array_Shuffle` _outrownames)
  (set `self.ForLoopIndexKilled` 1)
  (if (<= _forloopindexkilled 1) :!label _label_3
    (`|ExecutionSequence`
      (:`then_0`
        (goto _label))
      (:`then_1`
        (set `self.ForLoopIndexKilled` (+ _forloopindexkilled 1))
        (`KismetSystemLibrary.Delay` 0.02)
        (goto _label_3)))))

(event `Update`
  ;[1 1 1] Spawn planctons de base
  (if (< (`self.Index`) (`KismetArrayLibrary.Array_LastIndex` (stale `Spawn` _outrownames))) :!label _label_4
    (bind _returnvalue (`|GetDataTableRow` "/Game/Blueprints/Actors/Plancton_CSV.Plancton_CSV" (`KismetArrayLibrary.Array_Get` (stale `Spawn` _outrownames) (`self.Index`)))
      (:`then`
        (bind (_texture _normal _nom _famille _description _speed _type _level _nlevel _eleve) (break `/Game/Blueprints/Actors/STR_Plantons` _returnvalue))
        (if (select `/Game/Blueprints/Actors/EN_TypePlancton` _type :`NewEnumerator0` true :`NewEnumerator1` true :`NewEnumerator2` true :`NewEnumerator3` true :`NewEnumerator4` true :`NewEnumerator5` true :`NewEnumerator6` true :`NewEnumerator7` true :`NewEnumerator8` true :`NewEnumerator9` true :`NewEnumerator10` true :`NewEnumerator11` true :`NewEnumerator12` true)
          (bind _output_get (set `self.ActorLevel` _nlevel))
          (if (== _output_get (`self.TargetedLevel`))
            (`self.UpdateIndex`)
            (bind _returnvalue_2 (`|SpawnActorFromClass` "/Game/Blueprints/Actors/BP_MainPlancton.BP_MainPlancton_C" (`KismetMathLibrary.MakeTransform` (`KismetMathLibrary.MakeVector` (`KismetMathLibrary.RandomFloatInRange` -400.0 400.0) (`KismetMathLibrary.RandomFloatInRange` -800.0 800.0) _level) (struct) (5.0 5.0 1.0)) "Undefined" "OverrideRootScale" null _level (/ _speed 4.0) _texture _type _normal (`KismetTextLibrary.Conv_StringToText` _nom) (`KismetTextLibrary.Conv_StringToText` _famille) (`KismetTextLibrary.Conv_StringToText` _description) _nlevel null (`KismetTextLibrary.Conv_StringToText` _eleve) false "NewEnumerator0" (`self.PlasticGameMode`) 4.0 6.0 false 3.0 6.0 5))
            (`/Game/Blueprints/Actors/BP_MainPlancton.Opacity` _returnvalue_2 (`self.TargetedLevel`))
            (`/Game/Blueprints/Actors/BP_MainPlancton.Scaling` _returnvalue_2 true (`self.ZoomIn`) (stale `Spawn` Begin))
            (`/Game/Blueprints/Actors/BP_MainPlancton.Set all actors` _returnvalue_2 _returnvalue_2)
            (else
              (`self.UpdateIndex` :!label _label_5)
              (`self.Update`)))
          (else
            (goto _label_5)))))))

(event `Spawn`
  (params (TargetedLevel :type "/Game/Blueprints/Actors/EN_Level Enum") (ZoomIn :type Boolean) (Begin :type Boolean) (PlasticGameMode :type Boolean))
  (bind _forloopindex (`self.ForLoopIndex`))
  ;[1 1 1] Spawn planctons de base
  (set `self.ZoomIn` ZoomIn)
  (set `self.TargetedLevel` TargetedLevel)
  (set `self.Index` 0)
  (bind _outrownames (`DataTableFunctionLibrary.GetDataTableRowNames` "/Game/Blueprints/Actors/Plancton_CSV.Plancton_CSV"))
  (`KismetArrayLibrary.Array_Shuffle` _outrownames)
  (set `self.ForLoopIndex` 1)
  (if (<= _forloopindex 20) :!label _label_6
    (`|ExecutionSequence`
      (:`then_0`
        (goto _label_4))
      (:`then_1`
        (set `self.ForLoopIndex` (+ _forloopindex 1))
        (`KismetSystemLibrary.Delay` 0.05)
        (goto _label_6)))))

(event `Destroy`
  (params (ZoomIn :type Boolean))
  ;[1 1 1] Spawn planctons de base
  (bind _outactors (`GameplayStatics.GetAllActorsOfClass` "/Game/Blueprints/Actors/BP_MainPlancton.BP_MainPlancton_C"))
  (`/Game/Blueprints/Actors/BP_MainPlancton.Destroy` _outactors (`self.TargetedLevel`) ZoomIn))

(event `Plastica-Robota-Spawn`
  (params (TargetedLevel :type "/Game/Blueprints/Actors/EN_Level Enum") (ZValue :type "Float (double-precision)") (`Is Level` :type "/Game/Blueprints/Actors/EN_Level Enum") (ToSpawn :type Integer) (MinSpeed :type "Float (double-precision)") (MaxSpeed :type "Float (double-precision)") (Difficulty :type Integer))
  ;[1 1 1] Spawn Plastica Robota
  (bind _outactors (`GameplayStatics.GetAllActorsOfClass` "/Game/Blueprints/Actors/BP_MainPlancton.BP_MainPlancton_C"))
  (bind _returnvalue (`|GetDataTableRow` "/Game/Blueprints/Actors/Plancton_CSV.Plancton_CSV" "T_PLASTICAROBOTA")
    (:`then`
      (bind (_texture _normal _nom _famille _description _speed _type) (break `/Game/Blueprints/Actors/STR_Plantons` _returnvalue))
      (if (select `/Game/Blueprints/Actors/EN_TypePlancton` _type :`NewEnumerator14` true)
        (`|SpawnActorFromClass` "/Game/Blueprints/Actors/BP_MainPlancton.BP_MainPlancton_C" (`KismetMathLibrary.MakeTransform` (`KismetMathLibrary.MakeVector` (`KismetMathLibrary.RandomFloatInRange` -400.0 400.0) (`KismetMathLibrary.RandomFloatInRange` -800.0 800.0) ZValue) (struct) (5.0 5.0 1.0)) "Undefined" "OverrideRootScale" null ZValue (/ _speed 2.0) _texture _type _normal (`KismetTextLibrary.Conv_StringToText` _nom) (`KismetTextLibrary.Conv_StringToText` _famille) (`KismetTextLibrary.Conv_StringToText` _description) "NewEnumerator0" null "" false "NewEnumerator0" (`self.PlasticGameMode`) 4.0 6.0 false 3.0 6.0 Difficulty)))))

(event `UpdatePlastic`)

(event `Spawn-Plastico`
  (params (TargetedLevel :type "/Game/Blueprints/Actors/EN_Level Enum") (ZValue :type "Float (double-precision)") (`Is Level` :type "/Game/Blueprints/Actors/EN_Level Enum") (ToSpawn :type Integer) (MinSpeed :type "Float (double-precision)") (MaxSpeed :type "Float (double-precision)"))
  (bind _forloopindexplastico (`self.ForLoopIndexPlastico`))
  ;[1 1 1] Spawn Plasticoplanctons
  (set `self.PlasticoMinSpeed` MinSpeed)
  (set `self.PlasticoMaxSpeed` MaxSpeed)
  (set `self.PlasticoToSpawn` ToSpawn)
  (set `self.Zvalue` ZValue)
  (set `self.Is Level` `Is Level`)
  (set `self.TargetedLevel` TargetedLevel)
  (set `self.PlasticIndex` 0)
  (set `self.ForLoopIndexPlastico` 1)
  (if (<= _forloopindexplastico (`self.PlasticoToSpawn`)) :!label _label_7
    (`|ExecutionSequence`
      (:`then_0`
        (bind _returnvalue (`|GetDataTableRow` "/Game/Blueprints/Actors/Plancton_CSV.Plancton_CSV" (select `int` (`KismetMathLibrary.RandomIntegerInRange` 0 2) :`0` "T_PLASTICOPLANCTONS_01" :`1` "T_PLASTICOPLANCTONS_02" :`2` "T_PLASTICOPLANCTONS_01" :!type "Name"))
          (:`then`
            (set `self.SpawnedPlastico` (+ (`self.SpawnedPlastico`) 1))
            (bind (_texture _normal _nom _famille _description _speed _type _level _nlevel _eleve) (break `/Game/Blueprints/Actors/STR_Plantons` _returnvalue))
            (`|SpawnActorFromClass` "/Game/Blueprints/Actors/BP_MainPlancton.BP_MainPlancton_C" (`KismetMathLibrary.MakeTransform` (`KismetMathLibrary.MakeVector` (`KismetMathLibrary.RandomFloatInRange` -400.0 400.0) (`KismetMathLibrary.RandomFloatInRange` -400.0 400.0) (`self.Zvalue`)) (struct) (5.0 5.0 1.0)) "Undefined" "OverrideRootScale" null (`self.Zvalue`) _speed _texture _type _normal (`KismetTextLibrary.Conv_StringToText` _nom) (`KismetTextLibrary.Conv_StringToText` _famille) (`KismetTextLibrary.Conv_StringToText` _description) (`self.Is Level`) null (`KismetTextLibrary.Conv_StringToText` _eleve) false "NewEnumerator0" (`self.PlasticGameMode`) (`self.PlasticoMinSpeed`) (`self.PlasticoMaxSpeed`) true 3.0 6.0 5)
            (bind _outactors (`GameplayStatics.GetAllActorsOfClass` "/Game/Blueprints/Actors/BP_MainPlancton.BP_MainPlancton_C"))
            (`/Game/Blueprints/Actors/BP_MainPlancton.PlasticoThatSpawned` _outactors))))
      (:`then_1`
        (set `self.ForLoopIndexPlastico` (+ _forloopindexplastico 1))
        (`KismetSystemLibrary.Delay` 0.02)
        (goto _label_7)))))

(event `DestroyPlastico`
  (params (ZoomIn :type Boolean))
  ;[1 1 1] Spawn Plasticoplanctons
)

(fn `UpdateIndex`
  (set `self.Index` (+ (`self.Index`) 1))
  (return))

(fn `UpdateIndexKill`
  (set `self.KilledIndex` (+ (`self.KilledIndex`) 1))
  (return))

(fn `UpdateIndexPlastic`
  (set `self.PlasticIndex` (+ (`self.PlasticIndex`) 1))
  (return))

(fn `UserConstructionScript`)